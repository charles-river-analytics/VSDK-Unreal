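; BP_Button is an interactable push button that hands press through an EnterExitInteractionVolume component.
; When the volume's use finishes with a hand, it drives an InteractableSlider axis to the pressed position, or back to start if already pressed.
; Unless StayPressed is set, it returns automatically after the slider's movement time; otherwise it works as a toggle.
; Debug prints remain in the press logic.
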(event `self.EnterExitInteractionVolume.OnUseFinished`
  (params (InteractingActor :type "Actor Object Reference"))
  (bind _returnvalue (`InteractionVolume.IsHand` (`self.EnterExitInteractionVolume`) InteractingActor))
  (`KismetSystemLibrary.PrintString` "IsHand")
  (if _returnvalue
    (if (`self.bCurrentlyPressed`)
      (`self.ReturnButtonToStart`)
      (else
        (`KismetSystemLibrary.PrintString` "NotPressed")
        (`InteractableAxisControl.SetAxisValue` (`self.InteractableSlider`) 2 1 false)
        (set `self.bCurrentlyPressed` true)
        (if (not (`self.bStayPressed`))
          (`KismetSystemLibrary.Delay` (`InteractableAxisControl.movementTime` (`self.InteractableSlider`)))
          (`self.ReturnButtonToStart`))))))

(fn `ReturnButtonToStart`
  (`InteractableAxisControl.SetAxisValue` (`self.InteractableSlider`) 2 0 false)
  (set `self.bCurrentlyPressed` false))

(fn `UserConstructionScript`
  (`parent.UserConstructionScript`))