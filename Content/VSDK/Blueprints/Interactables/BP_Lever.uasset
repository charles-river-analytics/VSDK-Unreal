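; BP_Lever is a lever interactable in the VSDK that so far only prints debug feedback, with no lever behavior in its graphs.
; Its DefaultSelectComponent prints a message on select, and its DefaultGrabComponent prints the grabbing actor's display name on grab.
; BeginPlay, overlap and Tick are disabled stubs, and the construction script only calls its parent.
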(event `self.DefaultSelectComponent.OnSelect`
  (params (InteractableSelectSource :type "InteractableSelect Object Reference") (SelectingActor :type "Actor Object Reference"))
  (`KismetSystemLibrary.PrintString` "Select"))

(event `self.DefaultGrabComponent.OnGrab`
  (params (InteractableGrabSource :type "InteractableGrab Object Reference") (GrabbingActor :type "Actor Object Reference"))
  (`KismetSystemLibrary.PrintString` (`KismetSystemLibrary.GetDisplayName` GrabbingActor)))

(fn `UserConstructionScript`
  (`parent.UserConstructionScript`))