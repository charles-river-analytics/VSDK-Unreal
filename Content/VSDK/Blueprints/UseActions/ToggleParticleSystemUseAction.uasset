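; Use action that switches a particle system on its interactable owner on and off.
; On BeginPlay it fetches the owner's first ParticleSystemComponent and prints a debug string.
; TryUse activates that component without resetting it and TryUnuse deactivates it, each only when the component is valid.
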(event `self.TryUse`
  (params (UsingActor :type "Actor Object Reference"))
  (bind _particlesystem (`self.ParticleSystem`))
  (`/Engine/EditorBlueprintResources/StandardMacros.IsValid` _particlesystem
    (:`Is Valid`
      (`ActorComponent.Activate` _particlesystem false))))

(event `self.TryUnuse`
  (params (UnusingActor :type "Actor Object Reference"))
  (bind _particlesystem (`self.ParticleSystem`))
  (`/Engine/EditorBlueprintResources/StandardMacros.IsValid` _particlesystem
    (:`Is Valid`
      (`ActorComponent.Deactivate` _particlesystem))))

(event `self.BeginPlay`
  (bind _returnvalue (`self.GetInteractableOwner`))
  (set `self.ParticleSystem` (`Actor.GetComponentByClass` _returnvalue "/Script/Engine.ParticleSystemComponent"))
  (`KismetSystemLibrary.PrintString` null "Set PS"))