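; An interaction volume Blueprint that triggers use and finish actions from a counted number of actor enter or exit events.
; On BeginPlay it binds the enter and exit delegates, with UseOnEnter choosing which one counts.
; The first counted event calls UseVolume, each decrements the counter, and reaching zero calls FinishUseVolume.
; ResetOnFinish restores the counter so the cycle can repeat.
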(event `OnObjectExit_Event_0` :!signature `self.OnObjectExit`
  (params (InteractingActor :type "Actor Object Reference"))
  (if (not (`self.bUseOnEnter`))
    (`KismetSystemLibrary.PrintString` "Exit")
    (`self.CheckEnterExitCount` InteractingActor)))

(event `self.ReceiveBeginPlay`
  (set `self.currentEnterExitCount` (`self.enterExitCount`))
  (add `self.OnObjectEnter` (delegate `OnObjectEnter_Event_0`))
  (add `self.OnObjectExit` (delegate `OnObjectExit_Event_0`)))

(event `OnObjectEnter_Event_0` :!signature `self.OnObjectEnter`
  (params (InteractingActor :type "Actor Object Reference"))
  (if (`self.bUseOnEnter`)
    (`KismetSystemLibrary.PrintString` "Enter")
    (`self.CheckEnterExitCount` InteractingActor)))