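; Interaction volume that runs a timed use when an object enters it.
; The enter handler starts a timer of configurable duration and calls UseVolume; on expiry, TimerFinished calls FinishUseVolume and prints a debug message.
; The exit handler clears the timer and started flag, but BeginPlay binds it to OnObjectEnter alongside the enter handler.
; The started flag blocks restarts and is not reset on expiry.
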(event `self.ReceiveBeginPlay`
  (add `InteractionVolume.OnObjectEnter` (delegate `OnObjectEnter_Event_0`))
  (add `self.OnObjectEnter` (delegate `OnObjectExit_Event`)))

(event `OnObjectExit_Event` :!signature `self.OnObjectEnter`
  (params (InteractingActor :type "Actor Object Reference"))
  (if (`self.bHasTimerStarted`)
    (set `self.bHasTimerStarted` false)
    (`KismetSystemLibrary.K2_ClearAndInvalidateTimerHandle` (stale `OnObjectEnter_Event_0` _returnvalue))))

(event `OnObjectEnter_Event_0`
  (params (InteractingActor :type "Actor Object Reference"))
  (if (not (`self.bHasTimerStarted`))
    (bind _returnvalue (`KismetSystemLibrary.K2_SetTimer` null "TimerFinished" (`self.timerDurationSeconds`)))
    (set `self.bHasTimerStarted` true)
    (`InteractionVolume.UseVolume` InteractingActor)))

(fn `TimerFinished`
  (`InteractionVolume.FinishUseVolume` null)
  (`KismetSystemLibrary.PrintString` "Timer Finished"))