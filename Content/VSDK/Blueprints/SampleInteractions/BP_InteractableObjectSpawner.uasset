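; Sample interaction actor that keeps one grabbable item available at its location, replacing it whenever it is taken.
; On BeginPlay it spawns the configured class at its own transform and binds to that item's InteractableGrab grab event.
; If the item simulates physics, a PhysicsConstraint holds it in place.
; On grab it releases the constraint, unbinds, clears the reference and immediately spawns a replacement.
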(event `self.ReceiveBeginPlay`
  (`self.AttemptSpawn`))

(fn `AttemptSpawn`
  (`/Engine/EditorBlueprintResources/StandardMacros.IsValid` (`self.CurrentInteractable`)
    (:`Is Not Valid`
      (`self.SpawnItem`))))

(fn `Current Interactable Grabbed`
  (params (TheGrabObject :type "InteractableGrab Object Reference") (GrabbingActor :type "Actor Object Reference"))
  (`PhysicsConstraintComponent.SetConstrainedComponents` (`self.PhysicsConstraint`) null "None" null "None")
  (remove `InteractableGrab.OnInteractableGrab` (`self.GetComponentByClass` (`self.CurrentInteractable`) "/Script/VSDKInputPlugin.InteractableGrab") (`|CreateDelegate` :!event `Current Interactable Grabbed`))
  (set `self.CurrentInteractable` null)
  (`self.AttemptSpawn`))

(fn `SpawnItem`
  (bind _returnvalue (`|SpawnActorFromClass` (`self.InteractableToSpawn`) (`self.GetTransform`) "AdjustIfPossibleButAlwaysSpawn" "OverrideRootScale" null null))
  (bind _output_get (set `self.CurrentInteractable` _returnvalue))
  (add `InteractableGrab.OnInteractableGrab` (`self.GetComponentByClass` _output_get "/Script/VSDKInputPlugin.InteractableGrab") (`|CreateDelegate` :!event `Current Interactable Grabbed`))
  (if (`SceneComponent.IsSimulatingPhysics` (`Actor.RootComponent` (`self.CurrentInteractable`)) "None")
    (`PhysicsConstraintComponent.SetConstrainedComponents` (`self.PhysicsConstraint`) null "None" (`self.GetComponentByClass` (`self.CurrentInteractable`) "/Script/Engine.PrimitiveComponent") "None")))

(fn `UserConstructionScript`)